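; BP_Actions is the player input actor for click-to-move on BP_Grid: it spawns a PW_Hero and marks the hovered tile every tick.
; Left-clicking a tile of the matching type selects it and runs the grid's FindPath from the hero's tile.
; AIMoveTo walks the path tile by tile via a repeating timer, updating tile states.
; GetRotation snaps hero yaw from neighbor offsets, handling only hexagon grids.
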(event `self.ReceiveBeginPlay`
  (bind _returnvalue (`GameplayStatics.GetActorOfClass` "/Game/Blueprints/Core/Grid/BP_Grid.BP_Grid_C"))
  (set `self.Grid` _returnvalue)
  (`GameplayStatics.GetActorOfClass` "/Game/Blueprints/Core/Heros/PW_Hero.PW_Hero_C")
  (`self.EnableInput` (`GameplayStatics.GetPlayerController` 0))
  (bind _returnvalue_2 (`|SpawnActorFromClass` "/Game/Blueprints/Core/Heros/PW_Hero.PW_Hero_C" (`KismetMathLibrary.Conv_VectorToTransform` (`/Game/Blueprints/Core/Grid/BP_Grid.LocationBasedOnGridIndex` (`self.Grid`) (make `IntPoint` 10))) "AlwaysSpawn" "OverrideRootScale" null null))
  (set `self.Hero` _returnvalue_2))

(event `self.ReceiveTick`
  (params (DeltaSeconds :type "Float (single-precision)"))
  (`self.UpdateTileUnderCursor`))

(event `Key|LeftMouseButton`
  (params (Key :type "Key Structure"))
  (bind _hoveredtile (`self.HoveredTile`))
  (:`Pressed`
    (if (`|EnumEquality` (`.Type_6_C010CE7246E1DA6A035162837E7D0F75` (break `/Game/Blueprints/Core/Grid/Utilities/S_Tile_Data` (`BlueprintMapLibrary.Map_Find` (`/Game/Blueprints/Core/Grid/BP_Grid.GridTiles` (`self.Grid`)) (`self.HoveredTile`)))) "NewEnumerator1")
      (bind _states (`/Game/Blueprints/Core/Grid/BP_Grid.Get_TileState` (`self.Grid`) (`self.HoveredTile`)))
      (if (not (>= (`KismetArrayLibrary.Array_Find` _states "NewEnumerator2") 0))
        (`/Game/Blueprints/Core/Grid/BP_Grid.Remove_StateFromTile` (`self.Grid`) (`self.Selected_Tile`) "NewEnumerator2")
        (`/Game/Blueprints/Core/Grid/BP_Grid.Add_StateToTile` (`self.Grid`) _hoveredtile "NewEnumerator2")
        (`/Game/Blueprints/Core/Grid/BP_Grid.Remove_StateFromTile` (`self.Grid`) (`self.PreTile`) "NewEnumerator3")
        (`/Game/Blueprints/Core/Grid/BP_Grid.Remove_StateFromTile` (`self.Grid`) (`self.ToTile`) "NewEnumerator3")
        (set `self.Selected_Tile` _hoveredtile)
        (bind _tileindex (`/Game/Blueprints/Core/Grid/BP_Grid.Get_TileIndexFromWorldLocation` (`self.Grid`) (`self.K2_GetActorLocation` (`self.Hero`))))
        (`/Game/Blueprints/Core/Grid/BP_Grid.Find Path` (`self.Grid`) _tileindex (`self.Selected_Tile`) 0)
        (set `self.PreTile` (`|GetArrayItem` (`/Game/Blueprints/Core/Grid/BP_Grid.Path` (`self.Grid`))))
        (bind _output_get (set `self.ToTile` (`|GetArrayItem` (`/Game/Blueprints/Core/Grid/BP_Grid.Path` (`self.Grid`)) 1)))
        (`/Game/Blueprints/Core/Grid/BP_Grid.Add_StateToTile` (`self.Grid`) _output_get "NewEnumerator3")
        (`self.K2_SetActorRotation` (`self.Hero`) (`KismetMathLibrary.MakeRotator` 0.0 0.0 (`self.GetRotation` (`self.ToTile`) (`self.PreTile`))) false)
        (`|AIMoveTo` (`self.Hero`) (`/Game/Blueprints/Core/Grid/BP_Grid.LocationBasedOnGridIndex` (`self.Grid`) (`self.ToTile`)) null 0.0
          (:`then`
            (set `self.PreTile` (`self.ToTile`))
            (if (> (`KismetArrayLibrary.Array_Length` (`/Game/Blueprints/Core/Grid/BP_Grid.Path` (`self.Grid`))) 2)
              (set `self.Index` 2)
              (set `self.IsBreak` false)
              (`KismetSystemLibrary.K2_SetTimerDelegate` (delegate `loop1`) 0.3 (not (`self.IsBreak`))))))))))

(event `loop1`
  (if (not (`self.IsBreak`))
    (bind _output_get (set `self.ToTile` (`|GetArrayItem` (`/Game/Blueprints/Core/Grid/BP_Grid.Path` (`self.Grid`)) (`self.Index`))))
    (`/Game/Blueprints/Core/Grid/BP_Grid.Remove_StateFromTile` (`self.Grid`) (`self.PreTile`) "NewEnumerator3")
    (`/Game/Blueprints/Core/Grid/BP_Grid.Add_StateToTile` (`self.Grid`) _output_get "NewEnumerator3")
    (`self.K2_SetActorRotation` (`self.Hero`) (`KismetMathLibrary.MakeRotator` 0.0 0.0 (`self.GetRotation` (`self.ToTile`) (`self.PreTile`))) false)
    (`|AIMoveTo` (`self.Hero`) (`/Game/Blueprints/Core/Grid/BP_Grid.LocationBasedOnGridIndex` (`self.Grid`) (`self.ToTile`)) null 0.0
      (:`then`
        (set `self.Index` (+ (`self.Index`) 1))
        (set `self.PreTile` (`self.ToTile`))
        (if (>= (`self.Index`) (`KismetArrayLibrary.Array_Length` (`/Game/Blueprints/Core/Grid/BP_Grid.Path` (`self.Grid`))))
          (set `self.IsBreak` true)
          (set `self.Index` 0))))
    (else
      (`/Game/Blueprints/Core/Grid/BP_Grid.Remove_StateFromTile` (`self.Grid`) (`self.PreTile`) "NewEnumerator3"))))

(event `Key|RightMouseButton`
  (params (Key :type "Key Structure")))

(fn `GetRotation`
  (params (P1 :type "IntPoint Structure") (P2 :type "IntPoint Structure"))
  (returns (NewParam :type "Float (double-precision)"))
  (locals (NewLocalVar_0 :type "IntPoint Structure"))
  (bind _returnvalue (- P1 P2))
  (switch `/Game/Blueprints/Core/Grid/Grid_Shapes/E_Grid_Shape` (`/Game/Blueprints/Core/Grid/BP_Grid.Grid Shape` (`self.Grid`))
    (:`NewEnumerator2`
      (if (`KismetMathLibrary.Equal_IntPointIntPoint` _returnvalue (make `IntPoint` 0 2))
        (return 0.0)
        (elif (`KismetMathLibrary.Equal_IntPointIntPoint` _returnvalue (make `IntPoint` 1 1))
          (return -60.0)
          (elif (`KismetMathLibrary.Equal_IntPointIntPoint` _returnvalue (make `IntPoint` 1 -1))
            (return -120.0)
            (elif (`KismetMathLibrary.Equal_IntPointIntPoint` _returnvalue (make `IntPoint` 0 -2))
              (return -180.0)
              (elif (`KismetMathLibrary.Equal_IntPointIntPoint` _returnvalue (make `IntPoint` -1 -1))
                (return -240.0)
                (elif (`KismetMathLibrary.Equal_IntPointIntPoint` _returnvalue (make `IntPoint` -1 1))
                  (return -300.0))))))))))

(fn `UpdateTileUnderCursor`
  (bind _tileindex (`/Game/Blueprints/Core/Grid/BP_Grid.Get_TileIndexOnCursor` (`self.Grid`) 0))
  (if (!= _tileindex (`self.HoveredTile`))
    (`/Game/Blueprints/Core/Grid/BP_Grid.Remove_StateFromTile` (`self.Grid`) (`self.HoveredTile`) "NewEnumerator1")
    (set `self.HoveredTile` _tileindex)
    (`/Game/Blueprints/Core/Grid/BP_Grid.Add_StateToTile` (`self.Grid`) (`self.HoveredTile`) "NewEnumerator1")))

(fn `UserConstructionScript`)